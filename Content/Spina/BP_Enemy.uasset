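; BP_Enemy is a prototype AI enemy with a montage-driven melee attack and death handling.
; AttackStart and AttackEnd montage notifies bound a single sphere trace along the hand socket's movement.
; A hit calls ApplyDamage on the target's BP_CombatComponent, using that target component's own Damage value.
; On death, it calls Stop on the mesh, halts AI brain logic and disables capsule collision.
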(event OnDeath(BP_CombatComponent)
  ;[1 1 1] Mozliwe ze lepiej byloby obsluzyc smierc w behaviour tree w razie potrzeby przyszlego przywrocenia do zycia postaci
  (Audio|Components|Audio|Stop (Variables|Character|GetMesh))
  (AI|Logic|StopLogic (Variables|/Script/AIModule.AIController|GetBrainComponent (AI|GetAIController self)) "Death")
  (Collision|SetCollisionEnabled (Variables|Collision|GetCapsuleComponent) "NoCollision"))

(event EventMeleeAttack
  (bind _mesh (Variables|Character|GetMesh))
  (bind _returnvalue (Transformation|GetSocketLocation _mesh "middle_03_r_socket"))
  ;[1 1 1] Z racji redundancji kodu calosc tego mozna by przeniesc do jakiegos componentu (w prawdziwej grze to pewnie bylaby bron), natomiast z racji tego ze to mial byc prosty prototyp ktory pojdzie do kosza to nie ma sensu
  (bind _notifyname (Animation|Montage|PlayMontage _mesh "/Game/Spina/Attack_PrimaryA_Montage.Attack_PrimaryA_Montage")
    (:OnNotifyBegin
      (if (Utilities|Name|Equal(Name) _notifyname "AttackStart")
        (Variables|Default|SetAttackStartLocation _returnvalue)
        (elif (Utilities|Name|Equal(Name) _notifyname "AttackEnd")
          (bind _outhit (Collision|SphereTraceByChannel (Variables|Default|GetAttackStartLocation) _returnvalue 1e+01 "TraceTypeQuery2" false 0 "ForDuration" true "(R=1.000000,G=0.000000,B=0.000000,A=1.000000)" "(R=0.000000,G=1.000000,B=0.000000,A=1.000000)" 15.0))
          (if (.bBlockingHit (Collision|BreakHitResult _outhit))
            (Utilities|IsValid (Actor|GetComponentbyClass (.HitActor (Collision|BreakHitResult _outhit)) "/Game/Spina/BP_CombatComponent.BP_CombatComponent_C")
              (:Is%20Valid
                (Default|ApplyDamage (Actor|GetComponentbyClass (.HitActor (Collision|BreakHitResult _outhit)) "/Game/Spina/BP_CombatComponent.BP_CombatComponent_C") (Variables|/Game/Spina/BP_CombatComponent.BP_CombatComponent_C|GetDamage (Actor|GetComponentbyClass (.HitActor (Collision|BreakHitResult _outhit)) "/Game/Spina/BP_CombatComponent.BP_CombatComponent_C")))))))))))

(fn ConstructionScript)